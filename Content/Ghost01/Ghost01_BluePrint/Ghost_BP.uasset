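; Playable Ghost character with movement, jumping and combat skills: timed sprint with UI widget, line-traced forward teleport, montage attack and leap-then-dive dash.
; DoOnce nodes with delays gate repeat use, while timelines animate spring arm length during the dash.
; HItBoxTrace box-traces ahead to damage F-character pawns; taking damage interrupts montages and sets a hit flag.
; Death sets a flag and activates particle bursts; Y calls Res on the game mode.
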(event Custom|GetHitEnd
  (Variables|Default|SetGetHit? false))

(event Custom|Dead
  (Variables|Default|SetIsDead? true)
  (Components|Activation|SetActive (Variables|Default|GetZB) true false)
  (Utilities|FlowControl|Delay 0.2 :!label _label)
  (Components|Activation|SetActive (Variables|Default|Getbaozha) true false)
  (Utilities|FlowControl|Delay (Math|Random|RandomFloat))
  (Components|Activation|SetActive (Variables|Default|Getbaozha) false false)
  (for _index (range 0 3)
    (goto _label)))

(event Game|Damage|EventAnyDamage
  (params (Damage :type Float%20%28single-precision%29) (DamageType :type Damage%20Type%20Object%20Reference) (InstigatedBy :type Controller%20Object%20Reference) (DamageCauser :type Actor%20Object%20Reference))
  (Development|PrintString "Hello")
  (Animation|StopAnimMontage 0)
  (Variables|Default|SetGetHit? true))

(event Input|ActionEvents|InputActionJump
  (params (Key :type Key%20Structure :default "None"))
  ;[1 1 1] 基础移动跳跃
  (:Pressed
    (if (not (Variables|Sprint|GetIs%20Sprint)) :!label _label
      (Character|Jump)))
  (:Released
    (goto _label)))

(event Input|ActionEvents|InputActionAttack
  (params (Key :type Key%20Structure :default "None"))
  ;[1 1 1] 攻击
  (:Pressed
    (Networking|SwitchHasAuthority
      (:Authority
        (Utilities|FlowControl|DoOnce false :!label _label
          (:Completed
            (bind _returnvalue (Animation|PlayAnimMontage "/Game/Ghost01/Ghost01_AnimationBP/Ghost01_Attack.Ghost01_Attack" 1.0 "None"))
            (Utilities|FlowControl|Delay _returnvalue)
            (goto _label Reset)))))))

(event Input|AxisEvents|InputAxisTurn
  (params (AxisValue :type Float%20%28single-precision%29))
  ;[1 1 1] 基础移动跳跃
  (Pawn|Input|AddControllerYawInput AxisValue))

(event Input|AxisEvents|InputAxisLookUp
  (params (AxisValue :type Float%20%28single-precision%29))
  ;[1 1 1] 基础移动跳跃
  (Pawn|Input|AddControllerPitchInput AxisValue))

(event Input|AxisEvents|InputAxisMoveForward
  (params (AxisValue :type Float%20%28single-precision%29))
  ;[1 1 1] 基础移动跳跃
  (Pawn|Input|AddMovementInput (Math|Vector|GetForwardVector (Math|Rotator|MakeRotator 0.0 0.0 (.Yaw (Math|Rotator|BreakRotator (Pawn|GetControlRotation :!class /Script/Engine.Pawn))))) AxisValue false))

(event Input|AxisEvents|InputAxisMoveRight
  (params (AxisValue :type Float%20%28single-precision%29))
  ;[1 1 1] 基础移动跳跃
  (Pawn|Input|AddMovementInput (Math|Vector|GetRightVector (Math|Rotator|MakeRotator 0.0 0.0 (.Yaw (Math|Rotator|BreakRotator (Pawn|GetControlRotation :!class /Script/Engine.Pawn))))) AxisValue false))

(event Input|KeyboardEvents|1
  (params (Key :type Key%20Structure :default "None"))
  ;[1 1 1] 疾跑
  (:Pressed
    (Utilities|FlowControl|DoOnce false :!label _label
      (:Completed
        (CallFunction|SprintStart (Variables|Sprint|Getsprint%20speed))
        (bind _returnvalue (UserInterface|CreateWidget "/Game/Ghost01/Ghost01_BluePrint/Ghost01_sprint.Ghost01_sprint_C" (Game|GetPlayerController 0)))
        (UserInterface|Viewport|AddtoViewport _returnvalue 0)
        (Utilities|FlowControl|Delay 5.0)
        (CallFunction|SprintStop (Variables|Sprint|Getback%20speed))
        (goto _label Reset)))))

(event Input|KeyboardEvents|2
  (params (Key :type Key%20Structure :default "None"))
  ;[1 1 1] 瞬移
  (:Pressed
    (Utilities|FlowControl|DoOnce false :!label _label
      (:Completed
        (CallFunction|GhostTeleport)
        (Utilities|FlowControl|Delay 3.0)
        (goto _label Reset))))
  (:Released
    (goto _label)))

(event Input|KeyboardEvents|Q
  (params (Key :type Key%20Structure :default "None"))
  ;[1 1 1] 突进技能
  (:Pressed
    (Variables|Default|SetTuJin? true)
    (CallFunction|TuJinUP)
    (bind _新建轨迹_0 (Timeline|时间轴_0 Play)
      (:Update
        (Variables|/Script/Engine.SpringArmComponent|SetTargetArmLength (Variables|Default|GetSpringArm) _新建轨迹_0)
        (Utilities|FlowControl|Delay 0.75)
        (Variables|Default|SetTuJin? false)
        (CallFunction|TuJin)
        (Utilities|FlowControl|DoOnce false :!label _label
          (:Completed
            (Animation|PlayAnimMontage "/Game/Ghost01/Ghost01_AnimationBP/Ghost01_Attack.Ghost01_Attack" 1.0 "None")
            (Utilities|FlowControl|Delay 0.35)
            (bind _新建轨迹_0_2 (Timeline|时间轴_1 ReverseFromEnd)
              (:Update
                (Variables|/Script/Engine.SpringArmComponent|SetTargetArmLength (Variables|Default|GetSpringArm) _新建轨迹_0_2)
                (Utilities|FlowControl|Delay 1.0)
                (goto _label Reset)))))))))

(event Input|KeyboardEvents|Y
  (params (Key :type Key%20Structure :default "None"))
  (:Pressed
    (bind _asgame_mode_play (Utilities|Casting|CastToGameMode-play (Game|GetGameMode)))
    (Default|Res _asgame_mode_play)))

(fn ConstructionScript)

(fn SprintStart
  (params (max%20speed :type Float%20%28single-precision%29))
  (Variables|/Script/Engine.CharacterMovementComponent|SetMaxWalkSpeed (Variables|Character|GetCharacterMovement) max%20speed)
  (Variables|Sprint|SetIs%20Sprint true))

(fn SprintStop
  (params (max%20speed :type Float%20%28single-precision%29))
  (Variables|/Script/Engine.CharacterMovementComponent|SetMaxWalkSpeed (Variables|Character|GetCharacterMovement) max%20speed)
  (Variables|Sprint|SetIs%20Sprint false))

(fn GhostTeleport
  (bind _returnvalue (Transformation|GetActorForwardVector))
  (bind _returnvalue_2 (Transformation|GetActorLocation))
  (bind _teleport_range (Variables|Default|GetTeleport%20Range))
  (bind _returnvalue_3 (* _returnvalue _teleport_range))
  (bind _returnvalue_4 (+ _returnvalue_2 _returnvalue_3))
  (bind (_outhit _returnvalue_5) (Collision|LineTraceByChannel _returnvalue_2 _returnvalue_4 "TraceTypeQuery2" false 0 "ForDuration"))
  (if _returnvalue_5
    (Transformation|Teleport (.ImpactPoint (Collision|BreakHitResult _outhit)) "0, 0, 0")
    (else
      (Transformation|Teleport _returnvalue_4 "0, 0, 0"))))

(fn HItBoxTrace
  (bind _returnvalue (Transformation|GetActorLocation))
  (bind _outhit (Class|KismetSystemLibrary|BoxTraceSingleforObjects _returnvalue (+ (* (Transformation|GetActorForwardVector) (Variables|Default|GetHit%20Box%20Trace%20Range)) _returnvalue) "35.000000,35.000000,35.000000" "0, 0, 0" (Utilities|Array|MakeArray "ObjectTypeQuery3") false 0 "ForDuration" true))
  (bind _asf_character (Utilities|Casting|CastToF-character (.HitActor (Collision|BreakHitResult _outhit))))
  (Game|Damage|ApplyDamage _asf_character (Variables|Default|GetAttackDamage) 0 self))

(fn TuJin
  (bind _returnvalue (Transformation|GetActorForwardVector))
  (bind _returnvalue_2 (* _returnvalue 4e+03))
  (bind (_x _y _z) (Math|Vector|BreakVector _returnvalue_2))
  (Character|LaunchCharacter (Math|Vector|MakeVector _x _y (+ _z -1.8e+03)) false false))

(fn TuJinUP
  (bind _returnvalue (Transformation|GetActorForwardVector))
  (bind _returnvalue_2 (* _returnvalue 1.0))
  (bind (_x _y _z) (Math|Vector|BreakVector _returnvalue_2))
  (Character|LaunchCharacter (Math|Vector|MakeVector _x _y (+ _z 1.5e+03)) false false))