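; BP_inventory is an actor that stores items in a fixed number of slots, each holding an item class and amount.
; BeginPlay sizes the slot array, and helper functions query slots or find empty ones and partial stacks.
; Additem reads the class-default stackable flag, fills partial stacks before empty slots, and recurses to split overflow or place non-stackables singly.
; It returns any leftover as Reset, reporting Success even when stackables find no room.
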(event EventBeginPlay
  (Utilities|Array|Resize (Variables|Default|GetSlots) (Variables|Default|GetamountOfslots)))

(event Collision|EventActorBeginOverlap
  (params (OtherActor :type Actor%20Object%20Reference)))

(event EventTick
  (params (DeltaSeconds :type Float%20%28single-precision%29)))

(fn ConstructionScript)

(fn IsSlotEmpty
  (params (Index :type Integer))
  (return (not (Utilities|IsValidClass (.itemclass (Utilities|Struct|BreakS_inventoryslot (Utilities|Array|Get(acopy) (Variables|Default|GetSlots) Index)))))))

(fn GetitemInfoAtlndex
  (params (Index :type Integer))
  (bind _slots (Variables|Default|GetSlots))
  (bind _output (Utilities|Array|Get(acopy) _slots Index))
  (bind (_itemclass _amount) (Utilities|Struct|BreakS_inventoryslot _output))
  (if (Utilities|IsValidClass _itemclass)
    (return false (Utilities|GetClassDefaults _itemclass) _amount)
    (else
      (return true "" 0))))

(fn SearchEmptySlot
  (bind (_array_element _array_index) (Utilities|Array|ForEachLoopwithBreak (Variables|Default|GetSlots) :!label _label)
    (:LoopBody
      (if (not (Utilities|IsValidClass (.itemclass (Utilities|Struct|BreakS_inventoryslot _array_element))))
        (LocalVariables|SetLocalBool true)
        (LocalVariables|SetLocalIndex _array_index)
        (goto _label Break)))
    (:Completed
      (return (LocalVariables|GetLocalIndex) (LocalVariables|GetLocalBool)))))

(fn Additem
  (params (Amount :type Integer) (Class :type Item%20BP%20Class%20Reference))
  (LocalVariables|SetLocalAmount Amount)
  (LocalVariables|SetLocalClass Class)
  (if (.canbestacked (Utilities|Struct|BreakS_iteminfo (Utilities|GetClassDefaults Class)))
    (bind (_success _index) (CallFunction|SearchFreeStack (LocalVariables|GetLocalClass)))
    (if _success
      (bind _output_get (LocalVariables|SetFoundIndex _index))
      (if (> (+ (.amount (Utilities|Struct|BreakS_inventoryslot (Utilities|Array|Get(acopy) (Variables|Default|GetSlots) _output_get))) (LocalVariables|GetLocalAmount)) (Variables|Default|GetMaxStackSize))
        (LocalVariables|SetLocalAmount (- (+ (.amount (Utilities|Struct|BreakS_inventoryslot (Utilities|Array|Get(acopy) (Variables|Default|GetSlots) _output_get))) (LocalVariables|GetLocalAmount)) (Variables|Default|GetMaxStackSize)))
        (Utilities|Array|SetArrayElem (Variables|Default|GetSlots) (LocalVariables|GetFoundIndex) (Utilities|Struct|MakeS_inventoryslot (LocalVariables|GetLocalClass) (Variables|Default|GetMaxStackSize)))
        (bind _reset (CallFunction|Additem (LocalVariables|GetLocalAmount) (LocalVariables|GetLocalClass)))
        (return true _reset)
        (else
          (Utilities|Array|SetArrayElem (Variables|Default|GetSlots) (LocalVariables|GetFoundIndex) (Utilities|Struct|MakeS_inventoryslot (LocalVariables|GetLocalClass) (+ (.amount (Utilities|Struct|BreakS_inventoryslot (Utilities|Array|Get(acopy) (Variables|Default|GetSlots) _output_get))) (LocalVariables|GetLocalAmount))))
          (return true 0)))
      (else
        (bind (_index_2 _success_2) (CallFunction|SearchEmptySlot))
        (if _success_2
          (LocalVariables|SetFoundIndex _index_2)
          (if (> (LocalVariables|GetLocalAmount) (Variables|Default|GetMaxStackSize))
            (Utilities|Array|SetArrayElem (Variables|Default|GetSlots) (LocalVariables|GetFoundIndex) (Utilities|Struct|MakeS_inventoryslot (LocalVariables|GetLocalClass) (Variables|Default|GetMaxStackSize)))
            (bind _reset_2 (CallFunction|Additem (- (LocalVariables|GetLocalAmount) (Variables|Default|GetMaxStackSize)) (LocalVariables|GetLocalClass)))
            (return true _reset_2)
            (else
              (Utilities|Array|SetArrayElem (Variables|Default|GetSlots) (LocalVariables|GetFoundIndex) (Utilities|Struct|MakeS_inventoryslot (LocalVariables|GetLocalClass) (LocalVariables|GetLocalAmount)))
              (return true 0)))
          (else
            (return true (LocalVariables|GetLocalAmount))))))
    (else
      (bind (_index_3 _success_3) (CallFunction|SearchEmptySlot))
      (if _success_3
        (LocalVariables|SetFoundIndex _index_3)
        (Utilities|Array|SetArrayElem (Variables|Default|GetSlots) (LocalVariables|GetFoundIndex) (Utilities|Struct|MakeS_inventoryslot (LocalVariables|GetLocalClass) 1))
        ;[1 0.7231 0.5564] 同时获取多个时单个保存
        (if (> (LocalVariables|GetLocalAmount) 1)
          (bind _reset_3 (CallFunction|Additem (- (LocalVariables|GetLocalAmount) 1) (LocalVariables|GetLocalClass)))
          (return true _reset_3)
          (else
            (return true 0)))
        (else
          (return false (LocalVariables|GetLocalAmount)))))))

(fn SearchFreeStack
  (params (Class :type Item%20BP%20Class%20Reference))
  (bind (_array_element _array_index) (Utilities|Array|ForEachLoopwithBreak (Variables|Default|GetSlots) :!label _label)
    (:LoopBody
      (if (Utilities|IsValidClass (.itemclass (Utilities|Struct|BreakS_inventoryslot _array_element)))
        (if (and (< (.amount (Utilities|Struct|BreakS_inventoryslot _array_element)) (Variables|Default|GetMaxStackSize)) (== (.itemclass (Utilities|Struct|BreakS_inventoryslot _array_element)) Class))
          (LocalVariables|SetLocalBool true)
          (LocalVariables|SetLOcalIndex _array_index)
          (goto _label Break))))
    (:Completed
      (return (LocalVariables|GetLocalBool) (LocalVariables|GetLOcalIndex)))))