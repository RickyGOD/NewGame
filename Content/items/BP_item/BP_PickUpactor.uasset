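; BP_PickUpactor is an item pickup that adds a Class and Amount of item to the inventory of an F-character that touches it.
; Its Sphere overlap casts the other actor and calls Additem on that character's InventoryRef.
; On success, any leftover count (returned as Reset) becomes the pickup's new Amount, otherwise the actor destroys itself.
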(event OnComponentBeginOverlap(Sphere)
  (params (OverlappedComponent :type Primitive%20Component%20Object%20Reference) (OtherActor :type Actor%20Object%20Reference) (OtherComp :type Primitive%20Component%20Object%20Reference) (OtherBodyIndex :type Integer) (bFromSweep :type Boolean) (SweepResult :type Hit%20Result%20Structure%20%28by%20ref%29))
  (bind _asf_character (Utilities|Casting|CastToF-character OtherActor))
  (Utilities|IsValid _asf_character
    (:Is%20Valid
      (bind (_success _reset) (Default|Additem (Variables|/Game/Character/F-character.F-character_C|GetInventoryRef _asf_character) (Variables|Default|GetAmount) (Variables|Default|GetClass)))
      (if _success
        (if (> _reset 0)
          (Variables|Default|SetAmount _reset)
          (else
            (Actor|DestroyActor)))))))

(event EventBeginPlay)

(event Collision|EventActorBeginOverlap
  (params (OtherActor :type Actor%20Object%20Reference)))

(event EventTick
  (params (DeltaSeconds :type Float%20%28single-precision%29)))

(fn ConstructionScript)